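; BP_Monster is an enemy actor that triggers game over when it collides with the player.
; A capsule hit against the controlled pawn calls PlayerDied, guarded by IsPlayed.
; PlayerDied plays the death sound at the player's location, destroys the monster and shows the GameOver widget.
; It then switches to UI-only input with a visible cursor and clears IsMoving on the PlayerCharacter.
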(event OnComponentHit(CapsuleComponent)
  (params (HitComponent :type Primitive%20Component%20Object%20Reference) (OtherActor :type Actor%20Object%20Reference) (OtherComp :type Primitive%20Component%20Object%20Reference) (NormalImpulse :type Vector :default "0, 0, 0") (Hit :type Hit%20Result%20Structure%20%28by%20ref%29))
  (if (== OtherActor (Pawn|GetControlledPawn (Game|GetPlayerController 0)))
    (if (not (Variables|Default|GetIsPlayed))
      (CallFunction|PlayerDied (Transformation|GetActorLocation OtherActor)))))

(event Custom|PlayerDied
  (params (playerLoc :type Vector))
  (bind _returnvalue (Game|GetPlayerController 0))
  (Audio|PlaySoundatLocation "/Game/Yongchan/Monster/Sound/YouDied.YouDied" playerLoc "0, 0, 0" 0.5 1.0 0.0 0 0 0)
  (Actor|DestroyActor)
  (Variables|Default|SetIsPlayed true)
  (bind _returnvalue_2 (UserInterface|CreateWidget "/Game/Yongchan/GameOver.GameOver_C"))
  (UserInterface|Viewport|AddtoViewport _returnvalue_2 0)
  (Input|SetInputModeUIOnly _returnvalue 0 "DoNotLock")
  (Variables|/Script/Engine.PlayerController|SetbShowMouseCursor _returnvalue true)
  (bind _asplayer_character (Utilities|Casting|CastToPlayerCharacter (Game|Player|GetPlayerPawn 0)))
  (Variables|/Game/Doopaang/PlayerCharacter.PlayerCharacter_C|SetIsMoving _asplayer_character false))

(event EventBeginPlay)

(event Collision|EventActorBeginOverlap
  (params (OtherActor :type Actor%20Object%20Reference)))

(event EventTick
  (params (DeltaSeconds :type Float%20%28single-precision%29)))

(fn ConstructionScript)