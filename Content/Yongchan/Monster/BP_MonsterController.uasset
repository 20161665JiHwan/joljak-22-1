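; AI controller for Monster pawns that runs the BT_Monster behavior tree for patrolling and player detection.
; On BeginPlay it starts the tree and seeds blackboard keys for path looping, patrol direction and wait time from the monster's PatrolPath.
; AI perception updates set the CanSeePlayer key whenever a MODCharacter is sensed or lost.
; An older setup that assigned the player to a blackboard key is left disconnected.
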(event OnTargetPerceptionUpdated(AIPerception)
  (params (Actor :type Actor%20Object%20Reference) (Stimulus :type AI%20Stimulus%20Structure))
  (Utilities|Casting|CastToMODCharacter Actor)
  (AI|Components|Blackboard|SetValueasBool (AI|GetBlackboard 0) (Utilities|Name|MakeLiteralName "CanSeePlayer") (.bSuccessfullySensed (Utilities|Struct|BreakAIStimulus Stimulus))))

(event EventBeginPlay
  (bind _returnvalue (AI|GetBlackboard 0))
  (AI|RunBehaviorTree "/Game/Yongchan/Monster/BT_Monster.BT_Monster")
  (bind _asmonster (Utilities|Casting|CastToMonster (Pawn|GetControlledPawn)))
  (bind _output_get (Variables|Default|SetMyPawn _asmonster))
  (AI|Components|Blackboard|SetValueasBool (AI|GetBlackboard 0) (Utilities|Name|MakeLiteralName "PathLooping") (Variables|/Game/Yongchan/Monster/PatrolPath.PatrolPath_C|GetIsLooping (Variables|/Game/Yongchan/Monster/Monster.Monster_C|GetPatrolPath _output_get)))
  (Class|BlackboardComponent|SetValueasInt _returnvalue (Utilities|Name|MakeLiteralName "Direction") 1)
  (AI|Components|Blackboard|SetValueasFloat _returnvalue (Utilities|Name|MakeLiteralName "WaitTime") (Variables|/Game/Yongchan/Monster/PatrolPath.PatrolPath_C|GetWaitTime (Variables|/Game/Yongchan/Monster/Monster.Monster_C|GetPatrolPath (Variables|Default|GetMyPawn)))))

(event EventTick
  (params (DeltaSeconds :type Float%20%28single-precision%29)))

(fn ConstructionScript)