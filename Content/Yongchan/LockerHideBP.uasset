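; Hideable locker where the player escapes the monster, with a QTE when it comes close.
; Overlapping both trigger boxes enables Hide input, which animates the door and toggles view, collision, flashlight and, unless chased, AI sight.
; While hidden, a recursive delay loop applies clamped look input to the locker camera.
; A monster entering QTEBox starts a chase or patrol QTE; FailQTE opens the door and ejects the player.
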(event OnComponentBeginOverlap(Box)
  (params (OverlappedComponent :type Primitive%20Component%20Object%20Reference) (OtherActor :type Actor%20Object%20Reference) (OtherComp :type Primitive%20Component%20Object%20Reference) (OtherBodyIndex :type Integer) (bFromSweep :type Boolean) (SweepResult :type Hit%20Result%20Structure%20%28by%20ref%29))
  (Variables|Default|SetCanHidingRight true)
  (if (Variables|Default|GetCanHidingLeft)
    (if (Variables|Default|GetCanHidingRight)
      (bind _asplayer_character (Utilities|Casting|CastToPlayerCharacter OtherActor))
      (Variables|Default|SetAs%20Player%20Character _asplayer_character)
      (Input|EnableInput (Game|GetPlayerController 0))
      (Utilities|FlowControl|Gate true) ; enters at Open
    )))

(event OnComponentEndOverlap(Box)
  (params (OverlappedComponent :type Primitive%20Component%20Object%20Reference) (OtherActor :type Actor%20Object%20Reference) (OtherComp :type Primitive%20Component%20Object%20Reference) (OtherBodyIndex :type Integer))
  (bind _returnvalue (Game|GetPlayerController 0))
  (Variables|Default|SetCanHidingRight false)
  (Utilities|Casting|CastToPlayerCharacter OtherActor)
  (Input|DisableInput _returnvalue)
  (Utilities|FlowControl|Gate true) ; enters at Close
)

(event OnComponentBeginOverlap(QTEBox)
  (params (OverlappedComponent :type Primitive%20Component%20Object%20Reference) (OtherActor :type Actor%20Object%20Reference) (OtherComp :type Primitive%20Component%20Object%20Reference) (OtherBodyIndex :type Integer) (bFromSweep :type Boolean) (SweepResult :type Hit%20Result%20Structure%20%28by%20ref%29))
  (bind _returnvalue (Game|GetPlayerController 0))
  (if (Actor|ActorHasTag OtherActor "Monster")
    (bind _asplayer_character_controller (Utilities|Casting|CastToPlayerCharacterController (Game|GetPlayerController 0)))
    (if (not (Variables|/Game/Doopaang/PlayerCharacterController.PlayerCharacterController_C|GetDoingQTE _asplayer_character_controller))
      (if (Variables|Default|GetIsHiding) :!label _label
        (Utilities|FlowControl|Sequence
          (:then_0
            (bind _asbp_monster (Utilities|Casting|CastToBP_Monster OtherActor))
            (if (Variables|/Game/Yongchan/Monster/BP_Monster.BP_Monster_C|GetChase _asbp_monster)
              (bind _asplayer_character_controller_2 (Utilities|Casting|CastToPlayerCharacterController _returnvalue))
              (Default|ChasePlayer _asplayer_character_controller_2)
              (else
                (bind _asplayer_character_controller_3 (Utilities|Casting|CastToPlayerCharacterController _returnvalue))
                (Default|Patrol _asplayer_character_controller_3))))
          (:then_1
            (bind _asbp_monster_controller (Utilities|Casting|CastToBP_MonsterController (AI|GetAIController OtherActor)))
            (Default|ProgressingQTE _asbp_monster_controller)))
        (else
          (Utilities|FlowControl|Delay 0.2)
          (goto _label))))))

(event OnComponentBeginOverlap(Box1)
  (params (OverlappedComponent :type Primitive%20Component%20Object%20Reference) (OtherActor :type Actor%20Object%20Reference) (OtherComp :type Primitive%20Component%20Object%20Reference) (OtherBodyIndex :type Integer) (bFromSweep :type Boolean) (SweepResult :type Hit%20Result%20Structure%20%28by%20ref%29))
  (Variables|Default|SetCanHidingLeft true)
  (if (Variables|Default|GetCanHidingLeft)
    (if (Variables|Default|GetCanHidingRight)
      (bind _asplayer_character (Utilities|Casting|CastToPlayerCharacter (stale OnComponentBeginOverlap(Box) OtherActor)))
      (Variables|Default|SetAs%20Player%20Character _asplayer_character)
      (Input|EnableInput (Game|GetPlayerController 0))
      (Utilities|FlowControl|Gate true) ; enters at Open
    )))

(event OnComponentEndOverlap(Box1)
  (params (OverlappedComponent :type Primitive%20Component%20Object%20Reference) (OtherActor :type Actor%20Object%20Reference) (OtherComp :type Primitive%20Component%20Object%20Reference) (OtherBodyIndex :type Integer))
  (Variables|Default|SetCanHidingLeft false))

(event Custom|Move%20Camera
  (if (Variables|Default|GetIsHiding)
    (Transformation|SetRelativeRotation (Variables|Default|GetCamera) (Math|Rotator|MakeRotator 0.0 (* (stale Input|AxisEvents|InputAxisLookUp _output_get) -1.0) (stale Input|AxisEvents|InputAxisTurn _output_get)) false false)
    (Utilities|FlowControl|Delay 0.001)
    (CallFunction|MoveCamera)))

(event Custom|FailQTE
  (bind _locker_door (Variables|Default|GetLocker_Door))
  (Collision|SetCollisionEnabled _locker_door "NoCollision")
  (bind _doortrack (Timeline|타임라인_0 Play)
    (:Update
      (Transformation|SetRelativeRotation _locker_door (Math|Rotator|MakeRotator 0.0 0.0 (Math|Float|Lerp (Variables|Default|GetClose%20Angle) (Variables|Default|GetOpen%20Angle) _doortrack)) false false)
      (Utilities|FlowControl|Delay 0.8)
      (bind _asplayer_character (Utilities|Casting|CastToPlayerCharacter (Game|GetPlayerCharacter 0)))
      (Transformation|SetActorLocation _asplayer_character (+ (Transformation|GetActorLocation _asplayer_character) "15.000000, 0, 0") false false)
      (Class|AIPerceptionStimuliSourceComponent|RegisterforSense (Variables|/Game/Doopaang/PlayerCharacter.PlayerCharacter_C|GetAIPerceptionStimuliSource _asplayer_character) "/Script/AIModule.AISense_Sight")
      (Collision|SetActorEnableCollision _asplayer_character true)
      (bind _returnvalue (Actor|GetActorOfClass "/Game/Yongchan/Monster/BP_Monster.BP_Monster_C"))
      (Transformation|SetActorRotation (Math|Rotator|MakeRotator 0.0 0.0 (- (.yaw (Transformation|GetActorRotation _asplayer_character)) 1.8e+02)))
      (bind _asbp_monster_controller (Utilities|Casting|CastToBP_MonsterController (AI|GetAIController _returnvalue)))
      (Default|NotProgressingQTE _asbp_monster_controller))))

(event Input|ActionEvents|InputActionHide
  (params (Key :type Key%20Structure :default "None"))
  (:Pressed
    (bind _asplayer_character_controller (Utilities|Casting|CastToPlayerCharacterController (Game|GetPlayerController 0)))
    (if (not (Variables|/Game/Doopaang/PlayerCharacterController.PlayerCharacterController_C|GetDoingQTE _asplayer_character_controller))
      (Utilities|FlowControl|Gate true :!label _label
        (:Exit
          (Utilities|FlowControl|Sequence
            (:then_0
              (CallFunction|ToggleHide)
              (CallFunction|MoveCamera)
              (Utilities|FlowControl|Delay 0.2)
              (Input|EnableInput (Game|GetPlayerController 0))
              (goto _label Open))
            (:then_1
              (|OpenDoor))))))))

(event Input|AxisEvents|InputAxisLookUp
  (params (AxisValue :type Float%20%28single-precision%29))
  (if (Variables|Default|GetIsHiding)
    (bind _output_get (Variables|Default|SetPitch (Math|Float|Clamp(Float) (+ (Variables|Default|GetPitch) AxisValue) -4e+01 2e+01)))
    (else
      (Pawn|Input|AddControllerPitchInput (Variables|Default|GetAs%20Player%20Character) AxisValue))))

(event Input|AxisEvents|InputAxisTurn
  (params (AxisValue :type Float%20%28single-precision%29))
  (if (Variables|Default|GetIsHiding)
    (bind _output_get (Variables|Default|SetYaw (Math|Float|Clamp(Float) (+ (Variables|Default|GetYaw) AxisValue) -6e+01 6e+01)))
    (else
      (Pawn|Input|AddControllerYawInput (Variables|Default|GetAs%20Player%20Character) AxisValue))))

(fn ConstructionScript)

(fn ToggleHide
  (bind _returnvalue (Game|Player|GetPlayerPawn 0))
  (bind _returnvalue_2 (Game|GetPlayerController 0))
  (bind _as_player_character (Variables|Default|GetAs%20Player%20Character))
  (bind _aiperceptionstimulisource (Variables|/Game/Doopaang/PlayerCharacter.PlayerCharacter_C|GetAIPerceptionStimuliSource _as_player_character))
  (if (Variables|Default|GetIsHiding)
    (bind _asplayer_character_controller (Utilities|Casting|CastToPlayerCharacterController (Game|GetPlayerController 0)))
    (if (not (Variables|/Game/Doopaang/PlayerCharacterController.PlayerCharacterController_C|GetDoingQTE _asplayer_character_controller))
      (Variables|Default|SetIsHiding false)
      (Collision|SetActorEnableCollision _as_player_character true)
      (Game|Player|SetViewTargetwithBlend _returnvalue_2 _as_player_character 0.8 "VTBlend_Linear" 0.0 false)
      (Class|AIPerceptionStimuliSourceComponent|RegisterforSense _aiperceptionstimulisource "/Script/AIModule.AISense_Sight")
      (bind _asplayer_character (Utilities|Casting|CastToPlayerCharacter _returnvalue))
      (Variables|/Game/Doopaang/PlayerCharacter.PlayerCharacter_C|SetIsMoving _asplayer_character true)
      (Rendering|SetActorHiddenInGame (Variables|/Script/MansionOfDarkness.MODCharacter|Getflash _asplayer_character) false))
    (else
      (Variables|Default|SetIsHiding true)
      (Collision|SetActorEnableCollision _as_player_character false)
      (Game|Player|SetViewTargetwithBlend _returnvalue_2 self 0.8 "VTBlend_Linear" 0.0 false)
      (Utilities|FlowControl|Sequence
        (:then_0
          (bind _returnvalue_3 (Actor|GetActorOfClass "/Game/Yongchan/Monster/BP_Monster.BP_Monster_C"))
          (if (not (Variables|/Game/Yongchan/Monster/BP_Monster.BP_Monster_C|GetChase _returnvalue_3))
            (Class|AIPerceptionStimuliSourceComponent|UnregisterfromSense _aiperceptionstimulisource "/Script/AIModule.AISense_Sight")))
        (:then_1
          (bind _asplayer_character_2 (Utilities|Casting|CastToPlayerCharacter _returnvalue))
          (Variables|/Game/Doopaang/PlayerCharacter.PlayerCharacter_C|SetIsMoving _asplayer_character_2 false)
          (Rendering|SetActorHiddenInGame (Variables|/Script/MansionOfDarkness.MODCharacter|Getflash _asplayer_character_2) true))))))